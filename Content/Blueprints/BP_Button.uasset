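; VR push button actor that toggles an On/Off text label with a haptic pulse.
; An overlapping VRPawn enables input and recolours the knob's dynamic material; leaving resets position, colour and toggle latch.
; Grip input nudges the knob along Z by controller velocity sign; outside its travel range, it fires haptics and toggles once per overlap.
; The Motion assignment is unwired, and left grip checks right-hand trigger and hover actions.
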(event `self.ReceiveBeginPlay`
  (set `self.ButtonStart` (`SceneComponent.RelativeLocation` (`self.Button`)))
  (`TextRenderComponent.K2_SetText` (`self.TextRender`) (`self.Off`))
  (set `self.TextUI` false)
  (bind _returnvalue (`PrimitiveComponent.CreateDynamicMaterialInstance` (`self.Button`) 0 "/Game/Models/Materials/Mat_Knob.Mat_Knob" "None"))
  (set `self.DynamicMaterial` _returnvalue))

(event `self.Box.OnComponentBeginOverlap`
  (params (OverlappedComponent :type "PrimitiveComponent Object Reference") (OtherActor :type "Actor Object Reference") (OtherComp :type "PrimitiveComponent Object Reference") (OtherBodyIndex :type Integer) (bFromSweep :type Boolean) (SweepResult :type "HitResult Structure (by ref)"))
  (bind _returnvalue (`GameplayStatics.GetPlayerController` 0))
  (cast `/Game/VRTemplate/Blueprints/VRPawn` OtherActor)
  (`self.EnableInput` _returnvalue)
  (`EnhancedInputSubsystemInterface.AddMappingContext` (pcsubsystem `EnhancedInputLocalPlayerSubsystem` _returnvalue) "/Game/VRTemplate/Input/IMC_Project.IMC_Project" 0 (struct))
  (set `self.ActiveHand` OtherComp)
  (set `self.RightHand` (`KismetStringLibrary.Contains` (`KismetSystemLibrary.GetObjectName` OtherComp) "right"))
  (bind _asmotion_controller_component (cast `MotionControllerComponent` (`SceneComponent.GetAttachParent` (`SceneComponent.GetAttachParent` OtherComp))))
  (`MaterialInstanceDynamic.SetVectorParameterValue` (`self.DynamicMaterial`) "Colour" (`KismetMathLibrary.Conv_ColorToLinearColor` (`self.TargetColour`))))

(event `self.Box.OnComponentEndOverlap`
  (params (OverlappedComponent :type "PrimitiveComponent Object Reference") (OtherActor :type "Actor Object Reference") (OtherComp :type "PrimitiveComponent Object Reference") (OtherBodyIndex :type Integer))
  (bind _returnvalue (`GameplayStatics.GetPlayerController` 0))
  (cast `/Game/VRTemplate/Blueprints/VRPawn` OtherActor)
  (set `self.Switch` true)
  (`KismetSystemLibrary.MoveComponentTo` (`self.Button`) (`self.ButtonStart`))
  (`self.DisableInput` _returnvalue)
  (`EnhancedInputSubsystemInterface.RemoveMappingContext` (pcsubsystem `EnhancedInputLocalPlayerSubsystem` _returnvalue) "/Game/VRTemplate/Input/IMC_Project.IMC_Project" (struct))
  (`MaterialInstanceDynamic.SetVectorParameterValue` (`self.DynamicMaterial`) "Colour" (`KismetMathLibrary.Conv_ColorToLinearColor` (`self.DefaultColour`))))

(event `EnhancedInput|/Game/VRTemplate/Input/Actions/Project/IA_Grip_RIght`
  (params (ActionValue :type Boolean) (ElapsedSeconds :type "Float (double-precision)") (TriggeredSeconds :type "Float (double-precision)") (InputAction :type "InputAction Object Reference" :default "/Game/VRTemplate/Input/Actions/Project/IA_Grip_RIght.IA_Grip_RIght"))
  (:`Triggered`
    (if (not (`|GetInputActionValue`))
      (if (`|GetInputActionValue`)
        (if (`self.RightHand`)
          (`self.Button_Pressed`))))))

(event `EnhancedInput|/Game/VRTemplate/Input/Actions/Project/IA_Grip_Left`
  (params (ActionValue :type Boolean) (ElapsedSeconds :type "Float (double-precision)") (TriggeredSeconds :type "Float (double-precision)") (InputAction :type "InputAction Object Reference" :default "/Game/VRTemplate/Input/Actions/Project/IA_Grip_Left.IA_Grip_Left"))
  (:`Triggered`
    (if (not (`|GetInputActionValue`))
      (if (`|GetInputActionValue`)
        (if (not (`self.RightHand`))
          (`self.Button_Pressed`))))))

(fn `Button_Pressed`
  (bind _returnvalue (`GameplayStatics.GetPlayerController` 0))
  (if (`KismetMathLibrary.InRange_FloatFloat` (.z (`SceneComponent.RelativeLocation` (`self.Button`))) 7.5 100.0)
    (`SceneComponent.K2_AddLocalOffset` (`self.Button`) (`KismetMathLibrary.MakeVector` 0.0 0.0 (`KismetMathLibrary.SelectFloat` 1.0 -1.0 (> (.x (`MotionControllerComponent.GetLinearVelocity` (`self.motion`))) 0.0))) false false)
    (else
      ;[1 1 1] Play a haptic effect if the button is at its maximum position.
      (if (`self.RightHand`)
        (`PlayerController.PlayHapticEffect` _returnvalue "/Game/VRTemplate/Haptics/PistolFireHapticEffect.PistolFireHapticEffect" "Right" 1.0 false)
        (if (`self.Switch`)
          (if (`self.TextUI`)
            (`TextRenderComponent.K2_SetText` (`self.TextRender`) (`self.On`))
            (if (`self.TextUI`)
              (set `self.TextUI` false)
              (set `self.Switch` false)
              (else
                (set `self.TextUI` true)
                (set `self.Switch` false)))
            (else
              (`TextRenderComponent.K2_SetText` (`self.TextRender`) (`self.Off`))
              (if (`self.TextUI`)
                (set `self.TextUI` false)
                (set `self.Switch` false)
                (else
                  (set `self.TextUI` true)
                  (set `self.Switch` false))))))
        (else
          (`PlayerController.PlayHapticEffect` _returnvalue "/Game/VRTemplate/Haptics/PistolFireHapticEffect.PistolFireHapticEffect" "Left" 1.0 false)
          (if (`self.Switch`)
            (if (`self.TextUI`)
              (`TextRenderComponent.K2_SetText` (`self.TextRender`) (`self.On`))
              (if (`self.TextUI`)
                (set `self.TextUI` false)
                (set `self.Switch` false)
                (else
                  (set `self.TextUI` true)
                  (set `self.Switch` false)))
              (else
                (`TextRenderComponent.K2_SetText` (`self.TextRender`) (`self.Off`))
                (if (`self.TextUI`)
                  (set `self.TextUI` false)
                  (set `self.Switch` false)
                  (else
                    (set `self.TextUI` true)
                    (set `self.Switch` false)))))))))))

(fn `UserConstructionScript`)