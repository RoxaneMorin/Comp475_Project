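; BP_Knob is a VR knob that detects a pinching hand, though its action so far only prints that hand's relative rotation.
; VRPawn overlap on the collider toggles input and IMC_Project, and records the touching component, identifying right or left by its name.
; Button plus trigger on that hand counts as a pinch and calls KnobInAction.
; A dynamic material recolours the knob for default, targeted and active states.
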(event `self.ReceiveBeginPlay`
  ;[1 1 1] Set Dynamic Material
  (bind _returnvalue (`PrimitiveComponent.CreateDynamicMaterialInstance` (`self.SM_Knob`) 0 "/Game/Models/Materials/Mat_Knob.Mat_Knob" "None"))
  (set `self.DynamicMaterial` _returnvalue))

(event `self.ReceiveActorBeginOverlap`
  (params (OtherActor :type "Actor Object Reference")))

(event `self.ReceiveActorEndOverlap`
  (params (OtherActor :type "Actor Object Reference")))

(event `self.Knob_Collider.OnComponentBeginOverlap`
  (params (OverlappedComponent :type "PrimitiveComponent Object Reference") (OtherActor :type "Actor Object Reference") (OtherComp :type "PrimitiveComponent Object Reference") (OtherBodyIndex :type Integer) (bFromSweep :type Boolean) (SweepResult :type "HitResult Structure (by ref)"))
  (bind _returnvalue (`GameplayStatics.GetPlayerController` 0))
  ;[1 1 1] On ColliderBeginOverlap, make sure we are touching the VR Pawn.
  (cast `/Game/VRTemplate/Blueprints/VRPawn` OtherActor)
  (`KismetSystemLibrary.PrintString` "Knob Activated")
  (set `self.InUse` true)
  ;[1 1 1] Activate or Deactivate the Project Inputs.
  (`self.EnableInput` _returnvalue)
  (`EnhancedInputSubsystemInterface.AddMappingContext` (pcsubsystem `EnhancedInputLocalPlayerSubsystem` _returnvalue) "/Game/VRTemplate/Input/IMC_Project.IMC_Project" 1 (struct))
  ;[1 1 1] Update object colour
  (`MaterialInstanceDynamic.SetVectorParameterValue` (`self.DynamicMaterial`) "Colour" (`KismetMathLibrary.Conv_ColorToLinearColor` (`self.TargetColour`)))
  ;[1 1 1] Determine which hand is being used.
  (set `self.ActiveHand` OtherComp)
  (bind _output_get (set `self.UsingRightHand` (`KismetStringLibrary.Contains` (`KismetSystemLibrary.GetObjectName` OtherComp) "right")))
  (`KismetSystemLibrary.PrintString` (`KismetMathLibrary.SelectString` "Using the Right Hand" "Using the left Hand" _output_get)))

(event `self.Knob_Collider.OnComponentEndOverlap`
  (params (OverlappedComponent :type "PrimitiveComponent Object Reference") (OtherActor :type "Actor Object Reference") (OtherComp :type "PrimitiveComponent Object Reference") (OtherBodyIndex :type Integer))
  (bind _returnvalue (`GameplayStatics.GetPlayerController` 0))
  ;[1 1 1] On ColliderEndOverlap, make sure we were touching the VR Pawn.
  (cast `/Game/VRTemplate/Blueprints/VRPawn` OtherActor)
  (`KismetSystemLibrary.PrintString` "Knob Deactivated")
  (set `self.InUse` false)
  ;[1 1 1] Activate or Deactivate the Project Inputs.
  (`self.DisableInput` _returnvalue)
  (`EnhancedInputSubsystemInterface.RemoveMappingContext` (pcsubsystem `EnhancedInputLocalPlayerSubsystem` _returnvalue) "/Game/VRTemplate/Input/IMC_Project.IMC_Project" (struct))
  ;[1 1 1] Update object colour
  (`MaterialInstanceDynamic.SetVectorParameterValue` (`self.DynamicMaterial`) "Colour" (`KismetMathLibrary.Conv_ColorToLinearColor` (`self.DefaultColour`))))

(event `EnhancedInput|/Game/VRTemplate/Input/Actions/Project/IA_ButtonRight`
  (params (ActionValue :type Boolean) (ElapsedSeconds :type "Float (double-precision)") (TriggeredSeconds :type "Float (double-precision)") (InputAction :type "InputAction Object Reference" :default "/Game/VRTemplate/Input/Actions/Project/IA_ButtonRight.IA_ButtonRight"))
  (bind _returnvalue (`|GetInputActionValue`))
  ;[1 1 1] Handle Inputs
  (:`Triggered`
    (if _returnvalue
      (if (`self.UsingRightHand`)
        (`self.KnobInAction` :!label _label))))
  (:`Started`
    (if _returnvalue
      (`KismetSystemLibrary.PrintString` "Right Hand Pinch Started" :!label _label_2)
      (if (`self.UsingRightHand`)
        (`MaterialInstanceDynamic.SetVectorParameterValue` (`self.DynamicMaterial`) "Colour" (`KismetMathLibrary.Conv_ColorToLinearColor` (`self.ActiveColour`)))
        (goto _label))))
  (:`Completed`
    (`KismetSystemLibrary.PrintString` "Right Hand Pinch Done" :!label _label_3)
    (if (`self.UsingRightHand`)
      (`MaterialInstanceDynamic.SetVectorParameterValue` (`self.DynamicMaterial`) "Colour" (`KismetMathLibrary.Conv_ColorToLinearColor` (`self.TargetColour`))))))

(event `EnhancedInput|/Game/VRTemplate/Input/Actions/Project/IA_ButtonLeft`
  (params (ActionValue :type Boolean) (ElapsedSeconds :type "Float (double-precision)") (TriggeredSeconds :type "Float (double-precision)") (InputAction :type "InputAction Object Reference" :default "/Game/VRTemplate/Input/Actions/Project/IA_ButtonLeft.IA_ButtonLeft"))
  (bind _returnvalue (`|GetInputActionValue`))
  ;[1 1 1] Handle Inputs
  (:`Triggered`
    (if _returnvalue
      (if (not (`self.UsingRightHand`))
        (`self.KnobInAction` :!label _label_4))))
  (:`Started`
    (if _returnvalue
      (`KismetSystemLibrary.PrintString` "Left Hand Pinch Started" :!label _label_5)
      (if (not (`self.UsingRightHand`))
        (`MaterialInstanceDynamic.SetVectorParameterValue` (`self.DynamicMaterial`) "Colour" (`KismetMathLibrary.Conv_ColorToLinearColor` (`self.ActiveColour`)))
        (goto _label_4))))
  (:`Completed`
    (`KismetSystemLibrary.PrintString` "Right Hand Pinch Done" :!label _label_6)
    (if (not (`self.UsingRightHand`))
      (`MaterialInstanceDynamic.SetVectorParameterValue` (`self.DynamicMaterial`) "Colour" (`KismetMathLibrary.Conv_ColorToLinearColor` (`self.TargetColour`))))))

(event `EnhancedInput|/Game/VRTemplate/Input/Actions/Project/IA_TriggerRight`
  (params (ActionValue :type Boolean) (ElapsedSeconds :type "Float (double-precision)") (TriggeredSeconds :type "Float (double-precision)") (InputAction :type "InputAction Object Reference" :default "/Game/VRTemplate/Input/Actions/Project/IA_TriggerRight.IA_TriggerRight"))
  ;[1 1 1] Handle Inputs
  (:`Started`
    (if (`|GetInputActionValue`)
      (goto _label_2)))
  (:`Completed`
    (goto _label_3)))

(event `EnhancedInput|/Game/VRTemplate/Input/Actions/Project/IA_TriggerLeft`
  (params (ActionValue :type Boolean) (ElapsedSeconds :type "Float (double-precision)") (TriggeredSeconds :type "Float (double-precision)") (InputAction :type "InputAction Object Reference" :default "/Game/VRTemplate/Input/Actions/Project/IA_TriggerLeft.IA_TriggerLeft"))
  ;[1 1 1] Handle Inputs
  (:`Started`
    (if (`|GetInputActionValue`)
      (goto _label_5)))
  (:`Completed`
    (goto _label_6)))

(fn `KnobInAction`
  (`KismetSystemLibrary.PrintString` (`KismetStringLibrary.Conv_RotatorToString` (`SceneComponent.RelativeRotation` (`self.ActiveHand`)))))

(fn `UserConstructionScript`)